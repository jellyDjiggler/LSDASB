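; Game mode that sets up a two-character battle when play begins.
; Player starts tagged P1 and P2 each spawn a fighter chosen by the game instance's single CharacterClass, so both players get the same character.
; Player controller 0 possesses P1, while a newly spawned BasePlayerController possesses P2.
; The fighters are then linked as opponents, P2 is flagged flipped, and the battle HUD is shown.
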(event `self.ReceiveBeginPlay`
  (bind _player1 (`self.player1`))
  (bind _player2 (`self.player2`))
  (bind _outactors (`GameplayStatics.GetAllActorsOfClass` "/Script/Engine.PlayerStart"))
  (for _array_element _outactors
    (`self.SpawnPlayers` _array_element))
  (if (`KismetSystemLibrary.IsValid` (`self.player1`))
    (if (`KismetSystemLibrary.IsValid` (`self.player2`))
      (set `LSDASBCharacter.otherPlayer` _player2 _player1)
      (set `LSDASBCharacter.otherPlayer` _player1 _player2)
      (set `LSDASBCharacter.isFlipped` true _player2)
      (bind _returnvalue (`|CreateWidget` "/Game/LSD/Blueprints/Widgets/WBP_BattleHud.WBP_BattleHud_C" (`GameplayStatics.GetPlayerController` 0)))
      (`UserWidget.AddToViewport` _returnvalue 0))))

(fn `DetermineCharacterClass`
  (params (Transform :type "Transform Structure") (Actor :type "Actor Object Reference"))
  (returns (CharacterReference :type "LSDASBCharacter Object Reference"))
  (bind _asbase_game_instance (cast `BaseGameInstance` (`GameplayStatics.GetGameInstance`)))
  (switch `ECharacterClass` (`BaseGameInstance.characterClass` _asbase_game_instance)
    (:`VE_LloydMillsIII`
      (bind _returnvalue (`|SpawnActorFromClass` "/Game/LSD/Blueprints/Characters/L/BP_LloydMillsIII.BP_LloydMillsIII_C" Transform "Undefined" "OverrideRootScale" Actor null))
      (return _returnvalue))
    (:`VE_GavinTaylor`
      (bind _returnvalue_2 (`|SpawnActorFromClass` "/Game/LSD/Blueprints/Characters/L/BP_GavinTaylor.BP_GavinTaylor_C" Transform "Undefined" "OverrideRootScale" Actor null))
      (return _returnvalue_2))
    (:`VE_VonnHaring`
      (bind _returnvalue_3 (`|SpawnActorFromClass` "/Game/LSD/Blueprints/Characters/L/BP_VonnHaring.BP_VonnHaring_C" Transform "Undefined" "OverrideRootScale" Actor null))
      (return _returnvalue_3))
    (:`VE_LloydBlack`
      (bind _returnvalue_4 (`|SpawnActorFromClass` "/Game/LSD/Blueprints/Characters/L/BP_LloydBlack.BP_LloydBlack_C" Transform "Undefined" "OverrideRootScale" Actor null))
      (return _returnvalue_4))
    (:`VE_AikawaIshiki`
      (bind _returnvalue_5 (`|SpawnActorFromClass` "/Game/LSD/Blueprints/Characters/L/BP_AikawaIshiki.BP_AikawaIshiki_C" Transform "Undefined" "OverrideRootScale" Actor null))
      (return _returnvalue_5))
    (:`VE_SilverYamato`
      (bind _returnvalue_6 (`|SpawnActorFromClass` "/Game/LSD/Blueprints/Characters/L/BP_SilverYamato.BP_SilverYamato_C" Transform "Undefined" "OverrideRootScale" Actor null))
      (return _returnvalue_6))
    (:`VE_LeonMazura`
      (bind _returnvalue_7 (`|SpawnActorFromClass` "/Game/LSD/Blueprints/Characters/S/BP_LeonMazura.BP_LeonMazura_C" Transform "Undefined" "OverrideRootScale" Actor null))
      (return _returnvalue_7))
    (:`VE_Grey`
      (bind _returnvalue_8 (`|SpawnActorFromClass` "/Game/LSD/Blueprints/Characters/S/BP_Grey.BP_Grey_C" Transform "Undefined" "OverrideRootScale" Actor null))
      (return _returnvalue_8))
    (:`VE_RenzoFurea`
      (bind _returnvalue_9 (`|SpawnActorFromClass` "/Game/LSD/Blueprints/Characters/D/BP_RenzoFurea.BP_RenzoFurea_C" Transform "Undefined" "OverrideRootScale" Actor null))
      (return _returnvalue_9))))

(fn `SpawnPlayers`
  (params (Object :type "Actor Object Reference"))
  (bind _returnvalue (`self.GetTransform` Object))
  (bind _asplayer_start (cast `PlayerStart` Object))
  (bind _playerstarttag (`PlayerStart.PlayerStartTag` _asplayer_start))
  (if (== "P1" _playerstarttag)
    (bind _characterreference (`self.DetermineCharacterClass` (`self.GetTransform` Object) Object))
    (set `self.player1` _characterreference)
    (`Controller.Possess` (`GameplayStatics.GetPlayerController` 0) _characterreference)
    (elif (== _playerstarttag "P2")
      (bind _returnvalue_2 (`|SpawnActorFromClass` "/Script/LSDASB.BasePlayerController" _returnvalue "Undefined" "OverrideRootScale" null null))
      (bind _characterreference_2 (`self.DetermineCharacterClass` _returnvalue Object))
      (set `self.player2` _characterreference_2)
      (`Controller.Possess` _returnvalue_2 _characterreference_2))))

(fn `UserConstructionScript`)