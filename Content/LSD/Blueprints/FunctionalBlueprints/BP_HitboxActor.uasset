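; Fighting-game box actor that acts as a proximity hitbox, strike hitbox or hurtbox for either of two players.
; SpawnHitbox gives the display mesh a per-type material, moves it to the hitbox location, shows it, then runs a single overlap check.
; The check compares its owner to the game mode's Player1 to find the opponent's hurtbox.
; Overlapping proximity boxes notify the opponent, while strikes deal damage with stun, pushback and launch.
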(fn `CheckCollision`
  (bind _player2 (`LSDASBGameMode.player2` (`self.GameModeReference`)))
  (bind _player1 (`LSDASBGameMode.player1` (`self.GameModeReference`)))
  (bind _isplayerone (`self.DeterminePlayer`))
  (if _isplayerone
    (if (`self.IsOverlappingActor` (`LSDASBCharacter.hurtbox` _player2))
      (switch `EHitboxType` (`self.hitboxType`)
        (:`HB_PROXIMITY`
          (`LSDASBCharacter.CollidedWithProximityHitbox` _player2))
        (:`HB_STRIKE`
          (`LSDASBCharacter.TakeDamage` _player2 (`self.hitboxDamage`) (`self.hitstunTime`) (`self.blockstunTime`) (`self.pushbackDistance`) (`self.launchDistance`)))))
    (elif (`self.IsOverlappingActor` (`LSDASBCharacter.hurtbox` _player1))
      (switch `EHitboxType` (`self.hitboxType`)
        (:`HB_PROXIMITY`
          (`LSDASBCharacter.CollidedWithProximityHitbox` _player1))
        (:`HB_STRIKE`
          (`LSDASBCharacter.TakeDamage` _player1 (`self.hitboxDamage`) (`self.hitstunTime`) (`self.blockstunTime`) (`self.pushbackDistance`) (`self.launchDistance`)))))))

(fn `DeterminePlayer`
  (returns (isPlayerOne :type Boolean))
  (bind _aslsdasbgame_mode (cast `LSDASBGameMode` (`GameplayStatics.GetGameMode`)))
  (bind _output_get (set `self.GameModeReference` _aslsdasbgame_mode))
  (if (== (`LSDASBGameMode.player1` _output_get) (`self.GetOwner`))
    (return true)
    (else
      (return false))))

(fn `SpawnHitbox`
  (switch `EHitboxType` (`self.hitboxType`)
    (:`HB_PROXIMITY`
      (`PrimitiveComponent.SetMaterial` (`self.HitboxDisplay`) 0 "/Game/LSD/Art/Materials/M_ProximityHitbox.M_ProximityHitbox"))
    (:`HB_STRIKE`
      (`PrimitiveComponent.SetMaterial` (`self.HitboxDisplay`) 0 "/Game/LSD/Art/Materials/M_StrikeHitbox.M_StrikeHitbox"))
    (:`HB_HURTBOX`
      (`PrimitiveComponent.SetMaterial` (`self.HitboxDisplay`) 0 "/Game/LSD/Art/Materials/M_Hurtbox.M_Hurtbox")))
  (`SceneComponent.K2_SetWorldLocation` (`self.HitboxDisplay`) (`self.hitboxLocation`) false false)
  (`SceneComponent.SetVisibility` (`self.HitboxDisplay`) true false)
  (`self.CheckCollision`))

(fn `UserConstructionScript`)