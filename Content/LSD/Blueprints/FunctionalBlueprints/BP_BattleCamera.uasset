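; Two-player battle camera that follows both fighters along Y and Z at a fixed X.
; After a short delay, BeginPlay gets both players from BP_GameMode and spawns two BP_StageBoundary actors, placed once outside their starting positions.
; Each Tick moves the camera to a scaled average of the players' positions and sets a clamped FOV from their horizontal separation.
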(event `self.ReceiveBeginPlay`
  (`KismetSystemLibrary.Delay` 0.05)
  (bind _asbp_game_mode (cast `/Game/LSD/Blueprints/BP_GameMode` (`GameplayStatics.GetGameMode`)))
  (bind _player1 (`LSDASBGameMode.player1` _asbp_game_mode))
  (`/Engine/EditorBlueprintResources/StandardMacros.IsValid` _player1
    (:`Is Valid`
      (set `self.Player1Ref` _player1)
      (bind _player2 (`LSDASBGameMode.player2` _asbp_game_mode))
      (`/Engine/EditorBlueprintResources/StandardMacros.IsValid` _player2
        (:`Is Valid`
          (set `self.Player2Ref` _player2)
          (bind _returnvalue (`|SpawnActorFromClass` "/Game/LSD/Blueprints/FunctionalBlueprints/BP_StageBoundary.BP_StageBoundary_C" (`self.GetTransform`) "Undefined" "OverrideRootScale" null null))
          (set `self.LeftCameraEdge` _returnvalue)
          (bind _returnvalue_2 (`|SpawnActorFromClass` "/Game/LSD/Blueprints/FunctionalBlueprints/BP_StageBoundary.BP_StageBoundary_C" (`self.GetTransform`) "Undefined" "OverrideRootScale" null null))
          (set `self.RightCameraEdge` _returnvalue_2)
          (`self.SetCameraBoundaries`))))))

(event `self.ReceiveTick`
  (params (DeltaSeconds :type "Float (single-precision)"))
  (bind _player1ref (`self.Player1Ref`))
  (bind _player2ref (`self.Player2Ref`))
  (if (and (`KismetSystemLibrary.IsValid` _player1ref) (`KismetSystemLibrary.IsValid` _player2ref))
    (`self.K2_SetActorLocation` (`KismetMathLibrary.MakeVector` (.x (`self.K2_GetActorLocation`)) (/ (+ (.y (`self.K2_GetActorLocation` _player1ref)) (.y (`self.K2_GetActorLocation` _player2ref))) 1.8) (/ (+ (.z (`self.K2_GetActorLocation` _player1ref)) (.z (`self.K2_GetActorLocation` _player2ref))) 1.6)))
    (`CameraComponent.SetFieldOfView` (`self.CameraComponent`) (`KismetMathLibrary.FClamp` (`KismetMathLibrary.Abs` (* (- (.y (`self.K2_GetActorLocation` (`self.Player1Ref`))) (.y (`self.K2_GetActorLocation` (`self.Player2Ref`)))) 0.1)) 60.0 85.0))))

(fn `SetCameraBoundaries`
  (bind _returnvalue (- (.y (`self.K2_GetActorLocation` (`self.Player1Ref`))) 600.0))
  (bind _returnvalue_2 (+ (.y (`self.K2_GetActorLocation` (`self.Player2Ref`))) 600.0))
  (set `self.LeftMax` (- _returnvalue 300.0))
  (`self.K2_SetActorLocation` (`self.LeftCameraEdge`) (`KismetMathLibrary.MakeVector` (.x (`self.K2_GetActorLocation` (`self.Player1Ref`))) _returnvalue (.z (`self.K2_GetActorLocation` (`self.Player1Ref`)))) false false)
  (set `self.RightMax` (+ _returnvalue_2 300.0))
  (`self.K2_SetActorLocation` (`self.RightCameraEdge`) (`KismetMathLibrary.MakeVector` (.x (`self.K2_GetActorLocation` (`self.Player2Ref`))) _returnvalue_2 (.z (`self.K2_GetActorLocation` (`self.Player2Ref`)))) false false))

(fn `UserConstructionScript`)