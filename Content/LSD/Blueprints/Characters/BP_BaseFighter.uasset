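; Base fighter Blueprint for a two-player fighting game, which spawns and attaches its own hurtbox actor.
; It finds Player 2 through the game mode, retrying on Tick, and forwards shared-keyboard P2 input to that fighter.
; P1 key presses enter a timestamped input buffer that prunes stale entries.
; It also feeds per-player input icon stacks on the battle HUD, toggles the controls remap menu and sets palette materials.
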(event `self.ReceiveTick`
  (params (DeltaSeconds :type "Float (single-precision)"))
  (`/Engine/EditorBlueprintResources/StandardMacros.IsValid` (`self.Player2Reference`)
    (:`Is Not Valid`
      (bind _aslsdasbgame_mode (cast `LSDASBGameMode` (`GameplayStatics.GetGameMode`)))
      (bind _player2 (`LSDASBGameMode.player2` _aslsdasbgame_mode))
      (if (not (== _player2 self))
        (set `self.Player2Reference` _player2)))))

(event `self.ReceiveBeginPlay`
  (bind _aslsdasbgame_mode (cast `LSDASBGameMode` (`GameplayStatics.GetGameMode`)))
  (bind _player2 (`LSDASBGameMode.player2` _aslsdasbgame_mode))
  (if (not (== _player2 self))
    (set `self.Player2Reference` _player2))
  (bind _returnvalue (`|SpawnActorFromClass` "/Game/LSD/Blueprints/FunctionalBlueprints/BP_HurtboxActor.BP_HurtboxActor_C" (`self.GetTransform` (`PawnMovementComponent.GetPawnOwner` (`self.CharacterMovement`))) "Undefined" "OverrideRootScale" null null))
  (bind _output_get (set `self.hurtbox` _returnvalue))
  (`self.K2_AttachToActor` _output_get self "None" "SnapToTarget" "SnapToTarget" "SnapToTarget" true)
  (`self.SetOwner` _output_get self))

(event `InputAction|JumpP2`
  (params (Key :type "Key Structure"))
  (bind _player2reference (`self.Player2Reference`))
  (bind _player2reference_2 (`self.Player2Reference`))
  (:`Pressed`
    (`/Engine/EditorBlueprintResources/StandardMacros.IsValid` _player2reference_2
      (:`Is Valid`
        (`self.P2KeyboardJump` _player2reference_2))))
  (:`Released`
    (`/Engine/EditorBlueprintResources/StandardMacros.IsValid` _player2reference
      (:`Is Valid`
        (`self.P2KeyboardStopJumping` _player2reference)))))

(event `InputAction|LightAttackP2`
  (params (Key :type "Key Structure"))
  (bind _player2reference (`self.Player2Reference`))
  (:`Pressed`
    (`/Engine/EditorBlueprintResources/StandardMacros.IsValid` _player2reference
      (:`Is Valid`
        (`self.P2KeyboardLightAttack` _player2reference)))))

(event `InputAction|MediumAttackP2`
  (params (Key :type "Key Structure"))
  (bind _player2reference (`self.Player2Reference`))
  (:`Pressed`
    (`/Engine/EditorBlueprintResources/StandardMacros.IsValid` _player2reference
      (:`Is Valid`
        (`self.P2KeyboardMediumAttack` _player2reference)))))

(event `InputAction|HeavyAttackP2`
  (params (Key :type "Key Structure"))
  (bind _player2reference (`self.Player2Reference`))
  (:`Pressed`
    (`/Engine/EditorBlueprintResources/StandardMacros.IsValid` _player2reference
      (:`Is Valid`
        (`self.P2KeyboardHeavyAttack` _player2reference)))))

(event `InputAction|SpecialAttackP2`
  (params (Key :type "Key Structure"))
  (bind _player2reference (`self.Player2Reference`))
  (:`Pressed`
    (`/Engine/EditorBlueprintResources/StandardMacros.IsValid` _player2reference
      (:`Is Valid`
        (`self.P2KeyboardSpecialAttack` _player2reference)))))

(event `InputAxis|MoveRightP2`
  (params (AxisValue :type "Float (single-precision)"))
  (bind _player2reference (`self.Player2Reference`))
  (`/Engine/EditorBlueprintResources/StandardMacros.IsValid` _player2reference
    (:`Is Valid`
      (`self.P2KeyboardMoveRight` _player2reference AxisValue))))

(event `InputAction|CrouchP2`
  (params (Key :type "Key Structure"))
  (bind _player2reference (`self.Player2Reference`))
  (:`Pressed`
    (`/Engine/EditorBlueprintResources/StandardMacros.IsValid` _player2reference
      (:`Is Valid`
        (`self.StartCrouching` _player2reference))))
  (:`Released`
    (`/Engine/EditorBlueprintResources/StandardMacros.IsValid` _player2reference
      (:`Is Valid`
        (`self.StopCrouching` _player2reference)))))

(event `/Game/LSD/Blueprints/Interfaces/BPI_BasicFunctionInterface.SetHUDReferences`
  (bind _foundwidgets (`WidgetBlueprintLibrary.GetAllWidgetsOfClass` "/Game/LSD/Blueprints/Widgets/WBP_BattleHud.WBP_BattleHud_C"))
  (set `self.BattleHUDReference` (`|GetArrayItem` _foundwidgets)))

(event `self.AddInputIconToScreen`
  (params (_iconIndex :type Integer) (_shouldAddInput :type Boolean))
  (if _shouldAddInput
    (if (`self.isPlayerOne`)
      (`self.P1AddInputImage` _iconIndex)
      (else
        (`self.P2AddInputImage` _iconIndex)))))

(event `InputAction|OpenPauseMenu`
  (params (Key :type "Key Structure"))
  (bind _returnvalue (`GameplayStatics.GetPlayerController` 0))
  (:`Pressed`
    (`/Engine/EditorBlueprintResources/StandardMacros.FlipFlop`
      (:`A`
        (set `PlayerController.bShowMouseCursor` true _returnvalue)
        (bind _returnvalue_2 (`|CreateWidget` "/Game/LSD/Blueprints/Widgets/WBP_ControlsRemapMenu.WBP_ControlsRemapMenu_C" _returnvalue))
        (`UserWidget.AddToViewport` _returnvalue_2 0))
      (:`B`
        (set `PlayerController.bShowMouseCursor` false _returnvalue)
        (`Widget.RemoveFromParent` _returnvalue_2)))))

(event `InputAction|AddToInputBufferP1`
  (params (Key :type "Key Structure"))
  (bind _inputbuffer (`self.inputBuffer`))
  (:`Pressed`
    (for _array_element _inputbuffer
      (if (< (`.timeStamp` (break `InputInfo` _array_element)) (- (`GameplayStatics.GetTimeSeconds`) (`self.removeInputFromInputBufferTime`)))
        (`KismetArrayLibrary.Array_RemoveItem` _inputbuffer _array_element)))
    (`self.AddInputToInputBuffer` (make `InputInfo` (`KismetTextLibrary.Conv_TextToString` (`KismetInputLibrary.Key_GetDisplayName` Key)) (`GameplayStatics.GetTimeSeconds`)))))

(fn `P1AddInputImage`
  (params (IconIndex :type Integer))
  (locals (IconImageArray :type "Array of SlateBrush Structure"))
  (bind _returnvalue (`|CreateWidget` "/Game/LSD/Blueprints/Widgets/InputStack/WBP_InputStackIcon.WBP_InputStackIcon_C"))
  (`KismetArrayLibrary.Array_Insert` (`self.P1InputIcons`) _returnvalue)
  (`Image.SetBrush` (`/Game/LSD/Blueprints/Widgets/InputStack/WBP_InputStackIcon.InputIcon` _returnvalue) (`|GetArrayItem` (`local.IconImageArray`) IconIndex))
  (bind _battlehudreference (`self.BattleHUDReference`)
    (:`then`
      (bind _vb_inputstack (`/Game/LSD/Blueprints/Widgets/InputStack/WBP_InputStack.VB_InputStack` (`/Game/LSD/Blueprints/Widgets/WBP_BattleHud.P1Inputs` _battlehudreference)))
      (`PanelWidget.ClearChildren` _vb_inputstack)
      (for _array_element (`self.P1InputIcons`)
        (`PanelWidget.AddChild` _vb_inputstack _array_element)))
    (:`else`)))

(fn `P2AddInputImage`
  (params (IconIndex :type Integer))
  (locals (IconImageArray :type "Array of SlateBrush Structure"))
  (bind _returnvalue (`|CreateWidget` "/Game/LSD/Blueprints/Widgets/InputStack/WBP_InputStackIcon.WBP_InputStackIcon_C"))
  (`KismetArrayLibrary.Array_Insert` (`self.P2InputIcons`) _returnvalue)
  (`Image.SetBrush` (`/Game/LSD/Blueprints/Widgets/InputStack/WBP_InputStackIcon.InputIcon` _returnvalue) (`|GetArrayItem` (`local.IconImageArray`) IconIndex))
  (bind _battlehudreference (`self.BattleHUDReference`)
    (:`then`
      (bind _vb_inputstack (`/Game/LSD/Blueprints/Widgets/InputStack/WBP_InputStack.VB_InputStack` (`/Game/LSD/Blueprints/Widgets/WBP_BattleHud.P2Inputs` _battlehudreference)))
      (`PanelWidget.ClearChildren` _vb_inputstack)
      (for _array_element (`self.P2InputIcons`)
        (`PanelWidget.AddChild` _vb_inputstack _array_element)))
    (:`else`)))

(fn `SetCharacterPalette`
  (params (InMaterial :type "Material Object Reference"))
  (`PrimitiveComponent.SetMaterial` (`self.Mesh`) 0 InMaterial))

(fn `UserConstructionScript`)